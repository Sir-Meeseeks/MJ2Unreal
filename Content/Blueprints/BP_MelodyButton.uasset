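; BP_MelodyButton is an interactable button that plays a note and reports it to a PilarControl object, apparently as part of a melody puzzle.
; Overlapping its Box enables input for player controller 0, and ending the overlap disables it, without checking which actor overlaps.
; Pressing E plays NotePlayer and passes Note to PilarControl.AddNoteEvent.
; PilarControl's NotePlaying flag blocks further presses until the audio finishes.
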(event `self.Box.OnComponentBeginOverlap`
  (params (OverlappedComponent :type "PrimitiveComponent Object Reference") (OtherActor :type "Actor Object Reference") (OtherComp :type "PrimitiveComponent Object Reference") (OtherBodyIndex :type Integer) (bFromSweep :type Boolean) (SweepResult :type "HitResult Structure (by ref)"))
  (`self.EnableInput` (`GameplayStatics.GetPlayerController` 0)))

(event `self.Box.OnComponentEndOverlap`
  (params (OverlappedComponent :type "PrimitiveComponent Object Reference") (OtherActor :type "Actor Object Reference") (OtherComp :type "PrimitiveComponent Object Reference") (OtherBodyIndex :type Integer))
  (`self.DisableInput` (`GameplayStatics.GetPlayerController` 0)))

(event `self.NotePlayer.OnAudioFinished`
  (set `/Game/Blueprints/BP_PilarControl.NotePlaying` false (`self.PilarControl`)))

(event `Key|E`
  (params (Key :type "Key Structure"))
  (bind _pilarcontrol (`self.PilarControl`))
  (:`Pressed`
    (if (not (`/Game/Blueprints/BP_PilarControl.NotePlaying` (`self.PilarControl`)))
      (set `/Game/Blueprints/BP_PilarControl.NotePlaying` true _pilarcontrol)
      (`AudioComponent.Play` (`self.NotePlayer`) 0.0)
      (`/Game/Blueprints/BP_PilarControl.AddNote_Event` _pilarcontrol (`self.Note`)))))

(fn `UserConstructionScript`)