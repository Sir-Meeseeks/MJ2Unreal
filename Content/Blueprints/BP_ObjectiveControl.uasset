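; BP_ObjectiveControl tracks three level objectives and lights a torch for each one completed.
; SetObjective routes a number to the matching event, which activates its torch, sets that flag in the Objectives array and calls CheckForObjectives.
; CheckForObjectives tests all three flags, but its success branch is empty despite a comment about enabling an elevator.
; The Ambient audio component restarts whenever it finishes, looping the sound.
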(event `SetObjective1`
  ;[1 1 1] Set Objective 1
  (`/Game/Blueprints/BP_Torch_Large.Activate` (`self.Torch_1`))
  (`KismetArrayLibrary.Array_Set` (`self.Objectives`) 0 true)
  (`self.CheckForObjectives` :!label _label))

(event `CheckForObjectives`
  (bind _objectives (`self.Objectives`))
  ;[1 1 1] Enable Elevator if Objectives are satisfied
  (if (and (`|GetArrayItem` _objectives) (`|GetArrayItem` _objectives 1) (`|GetArrayItem` _objectives 2))
    _))

(event `SetObjective`
  (params (Objective :type Integer))
  ;[1 1 1] ReRoute Objective Event
  (switch `int` Objective
    (:`1`
      (`self.SetObjective1`))
    (:`2`
      (`self.SetObjective2`))
    (:`3`
      (`self.SetObjective3`))))

(event `SetObjective2`
  ;[1 1 1] Set Objective 2
  (`/Game/Blueprints/BP_Torch_Large.Activate` (`self.Torch_2`))
  (`KismetArrayLibrary.Array_Set` (`self.Objectives`) 1 true)
  (goto _label))

(event `self.Ambient.OnAudioFinished`
  (`AudioComponent.Play` (`self.Ambient`) 0.0))

(event `SetObjective3`
  ;[1 1 1] Set Objective 1
  (`/Game/Blueprints/BP_Torch_Large.Activate` (`self.Torch_3`))
  (`KismetArrayLibrary.Array_Set` (`self.Objectives`) 2 true)
  (goto _label))

(fn `UserConstructionScript`)