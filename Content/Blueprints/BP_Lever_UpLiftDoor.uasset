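; Interactive lever that the player toggles with the E key to trigger a linked door's move event.
; Overlapping the collision component enables input on the actor for the first player controller, and leaving disables it.
; Each pull flips the Pulled state, plays a grinding gear sound and runs one rotation timeline forward or in reverse.
; A BeingPulled flag blocks further pulls until the timeline finishes.
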(event `self.CollisionComponent.OnComponentBeginOverlap`
  (params (OverlappedComponent :type "PrimitiveComponent Object Reference") (OtherActor :type "Actor Object Reference") (OtherComp :type "PrimitiveComponent Object Reference") (OtherBodyIndex :type Integer) (bFromSweep :type Boolean) (SweepResult :type "HitResult Structure (by ref)"))
  (`self.EnableInput` (`GameplayStatics.GetPlayerController` 0)))

(event `self.CollisionComponent.OnComponentEndOverlap`
  (params (OverlappedComponent :type "PrimitiveComponent Object Reference") (OtherActor :type "Actor Object Reference") (OtherComp :type "PrimitiveComponent Object Reference") (OtherBodyIndex :type Integer))
  (`self.DisableInput` (`GameplayStatics.GetPlayerController` 0)))

(event `Key|E`
  (params (Key :type "Key Structure"))
  (:`Pressed`
    (if (not (`self.BeingPulled`))
      (set `self.BeingPulled` true)
      (if (`self.Pulled`)
        (set `self.Pulled` false)
        (`AudioComponent.Play` (`self.grindingGear`) 6.05)
        (`/Game/Blueprints/BP_UpliftDoor.MoveDoor_Event` (`self.DoorToOpen`))
        (bind (_direction _leverrotation) (`Timeline|LeverRotationOff` :!via `ReverseFromEnd` :!label _label)
          (:`Update`
            (`SceneComponent.K2_SetRelativeRotation` (`self.Lever`) (`KismetMathLibrary.MakeRotator` 0.0 _leverrotation) false false))
          (:`Finished`
            (set `self.BeingPulled` false)))
        (else
          (set `self.Pulled` true)
          (`AudioComponent.Play` (`self.grindingGear`) 6.05)
          (`/Game/Blueprints/BP_UpliftDoor.MoveDoor_Event` (`self.DoorToOpen`))
          (goto _label :!via `PlayFromStart`))))))

(fn `UserConstructionScript`
  (set `self.BeingPulled` false)
  (set `self.Pulled` false)
  (set `self.JustBeenPulled` false))