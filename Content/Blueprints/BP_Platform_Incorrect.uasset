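; BP_Platform_Incorrect is a trap platform, the wrong choice among platforms, that drops when something enters its trigger box.
; Any Box overlap turns on physics simulation on the Cube, with no check on the overlapping actor.
; DisguiseColor_Event applies the M_Jeroglyphics material to the Cube to disguise it.
; Restart stops physics and returns the Cube to the world transform saved in the construction script.
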(event `self.Box.OnComponentBeginOverlap`
  (params (OverlappedComponent :type "PrimitiveComponent Object Reference") (OtherActor :type "Actor Object Reference") (OtherComp :type "PrimitiveComponent Object Reference") (OtherBodyIndex :type Integer) (bFromSweep :type Boolean) (SweepResult :type "HitResult Structure (by ref)"))
  (`PrimitiveComponent.SetSimulatePhysics` (`self.Cube`) true))

(event `DisguiseColor_Event`
  (`PrimitiveComponent.SetMaterial` (`self.Cube`) 0 "/Game/Materials/M_Jeroglyphics.M_Jeroglyphics"))

(event `Restart`
  (bind _cube (`self.Cube`))
  (`PrimitiveComponent.SetSimulatePhysics` _cube false)
  (`SceneComponent.K2_SetWorldTransform` _cube (`self.InitialTransform`) false false))

(fn `UserConstructionScript`
  (set `self.InitialTransform` (`SceneComponent.K2_GetComponentToWorld` (`self.Cube`)))
  (set `self.InitialLocation` (`self.K2_GetActorLocation`)))