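; BP_LateralDoor is a sliding door that toggles open and closed along the X axis each time its MoveDoor event runs.
; MoveDoor flips DoorIsOpen, plays the moving rock sound, and plays the Move timeline forward to open or in reverse to close.
; The timeline offsets the static mesh's relative X from InitialPosition, which the construction script captures from the actor's world location while resetting the door to closed.
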(event `MoveDoor`
  (if (`self.DoorIsOpen`)
    (`AudioComponent.Play` (`self.MovingRockPlayer`) 0.0)
    (set `self.DoorIsOpen` false)
    (bind (_direction _movedoorfloat) (`Timeline|Move` :!via `ReverseFromEnd` :!label _label)
      (:`Update`
        (`SceneComponent.K2_SetRelativeLocation` (`self.StaticMeshComponent`) (`KismetMathLibrary.MakeVector` (+ _movedoorfloat (.x (`self.InitialPosition`))) (.y (`self.InitialPosition`)) (.z (`self.InitialPosition`))) false false)))
    (else
      (`AudioComponent.Play` (`self.MovingRockPlayer`) 0.0)
      (set `self.DoorIsOpen` true)
      (goto _label :!via `PlayFromStart`))))

(fn `UserConstructionScript`
  (set `self.DoorIsOpen` false)
  (set `self.InitialPosition` (`self.K2_GetActorLocation`)))