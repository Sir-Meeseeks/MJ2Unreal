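; BP_MovingPlatform3 is a moving platform actor meant to offset itself along Y and Z from its placed position.
; The construction script caches the world location as InitialLocation.
; The MoveY timeline update adds both MoveY and MoveZ track values to it and sets the relative location without sweeping.
; No event in the graph calls either timeline, and MoveZ has no update logic of its own.
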(fn `UserConstructionScript`
  (set `self.InitialLocation` (`self.K2_GetActorLocation`)))