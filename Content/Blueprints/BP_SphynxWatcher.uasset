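; BP_SphynxWatcher is a melody puzzle controller that checks incoming notes against stored sequences to open pillars.
; AddNote_Event routes notes by MelodyNumber to level 1 or 2 checks, which advance a shared index and reset it on a wrong note.
; A completed sequence opens its pillar, plays MelodyPlayer and advances MelodyNumber; melody 3 has no note check.
; Separate events swap the loaded sound or play it once as a preview.
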(event `SetMelody2`
  ;[1 1 1] Change melodies
  (`AudioComponent.SetSound` (`self.MelodyPlayer`) "/Game/Sounds/Melodies/nivell-2.nivell-2"))

(event `PlayMelody_Event`
  ;[1 1 1] Plays the current melody loaded.
  (if (not (`self.AlreadyPlayed`))
    (`AudioComponent.Play` (`self.MelodyPlayer`) 0.0)
    (set `self.AlreadyPlayed` true)))

(event `AddNote_Event`
  (params (NoteSent :type Integer))
  ;[1 1 1] Switch between melodies.
  (switch `int` (`self.MelodyNumber`)
    (:`1`
      (`self.AddNoteNivell1` NoteSent))
    (:`2`
      (`self.AddNoteNivell2` NoteSent))))

(event `SetMelody3`
  ;[1 1 1] Change melodies
  (`AudioComponent.SetSound` (`self.MelodyPlayer`) "/Game/Sounds/Melodies/nivell-3.nivell-3"))

(event `self.MelodyPlayer.OnAudioFinished`
  ;[1 1 1] Plays the current melody loaded.
  (set `self.NotePlaying` false))

(event `AddNoteNivell1`
  (params (Note :type Integer))
  (bind _notecounterinarray (`self.NoteCounterInArray`))
  ;[1 1 1] Melody 1 sequence
  (if (== Note (`|GetArrayItem` (`self.Nivell1Notes`) (`self.NoteCounterInArray`)))
    (if (== (- (`KismetArrayLibrary.Array_Length` (`self.Nivell1Notes`)) 1) _notecounterinarray)
      (set `self.NotePlaying` true)
      (`/Game/Blueprints/BP_MovingPilar.OpenPilar_Event` (`self.Pilar1`))
      (`AudioComponent.Play` (`self.MelodyPlayer`) 0.0)
      (set `self.MelodyNumber` 2)
      (else
        (bind _result (`/Engine/EditorBlueprintResources/StandardMacros.IncrementInt` _notecounterinarray)
          (:`  `
            (set `self.NoteCounterInArray` _result)))))
    (else
      (set `self.NoteCounterInArray` 0))))

(event `AddNoteNivell2`
  (params (Note :type Integer))
  (bind _notecounterinarray (`self.NoteCounterInArray`))
  ;[1 1 1] Melody 1 sequence
  (if (== Note (`|GetArrayItem` (`self.Nivell2Notes`) (`self.NoteCounterInArray`)))
    (if (== (- (`KismetArrayLibrary.Array_Length` (`self.Nivell2Notes`)) 1) _notecounterinarray)
      (set `self.NotePlaying` true)
      (`/Game/Blueprints/BP_MovingPilar.OpenPilar_Event` (`self.Pilar2`))
      (`AudioComponent.Play` (`self.MelodyPlayer`) 0.0)
      (set `self.MelodyNumber` 3)
      (else
        (bind _result (`/Engine/EditorBlueprintResources/StandardMacros.IncrementInt` _notecounterinarray)
          (:`  `
            (set `self.NoteCounterInArray` _result)))))
    (else
      (set `self.NoteCounterInArray` 0))))

(fn `UserConstructionScript`
  (set `self.MelodyNumber` 1)
  (set `self.AlreadyPlayed` false)
  (set `self.OnErrorAnimation` false)
  (set `self.NoteCounterInArray` 0)
  (set `self.NotePlaying` false))