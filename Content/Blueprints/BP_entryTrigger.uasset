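; Entry trigger volume that disguises the color of every PlataformaVermella platform in the level.
; The first overlap starts a TargetTime countdown in Tick, which keeps running because leaving never restores OutOfTrigger.
; Expiry, or leaving before it, sets DisguiseDone and calls DisguiseColorEvent on all those platforms.
; Tick does not check DisguiseDone, so it repeats that call every frame once the time is below zero.
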(event `self.ReceiveTick`
  (params (DeltaSeconds :type "Float (single-precision)"))
  (if (not (`self.OutOfTrigger`))
    (bind _output_get (set `self.targetTime` (- (`self.targetTime`) DeltaSeconds)))
    (if (< _output_get 0.0) :!label _label
      (set `self.DisguiseDone` true :!label _label_2)
      (bind _outactors (`GameplayStatics.GetAllActorsOfClass` (`self.PlataformaVermella`)))
      (for _array_element _outactors
        (`/Game/Blueprints/BP_Platform_Incorrect.DisguiseColor_Event` _array_element)))))

(event `self.CollisionComponent.OnComponentBeginOverlap`
  (params (OverlappedComponent :type "PrimitiveComponent Object Reference") (OtherActor :type "Actor Object Reference") (OtherComp :type "PrimitiveComponent Object Reference") (OtherBodyIndex :type Integer) (bFromSweep :type Boolean) (SweepResult :type "HitResult Structure (by ref)"))
  (set `self.OutOfTrigger` false)
  (if (`self.FirstTimeEnter`)
    (set `self.FirstTimeEnter` false)
    (if (not (`self.DisguiseDone`))
      (goto _label))))

(event `self.CollisionComponent.OnComponentEndOverlap`
  (params (OverlappedComponent :type "PrimitiveComponent Object Reference") (OtherActor :type "Actor Object Reference") (OtherComp :type "PrimitiveComponent Object Reference") (OtherBodyIndex :type Integer))
  (if (not (`self.DisguiseDone`))
    (goto _label_2)))

(fn `UserConstructionScript`
  (set `self.OutOfTrigger` true)
  (set `self.FirstTimeEnter` true)
  (set `self.DisguiseDone` false))