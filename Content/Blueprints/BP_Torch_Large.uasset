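; BP_Torch_Large is a large torch with a Fire component and a Light component.
; Activate shows the fire but hides the light.
; A Flicker timeline that would drive the light's green channel and intensity is never run.
; Tick only resets a Timer on a randomized threshold, and the construction script initializes that Timer and a MinColor value that is not read.
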(event `self.ReceiveTick`
  (params (DeltaSeconds :type "Float (single-precision)"))
  (if (> (+ DeltaSeconds (`self.Timer`)) (* 0.05 (`KismetMathLibrary.RandomFloat`)))
    (set `self.Timer` 0.0)))

(event `Activate`
  (`SceneComponent.SetVisibility` (`self.Fire`) true false)
  (`SceneComponent.SetVisibility` (`self.Light`) false false))

(fn `UserConstructionScript`
  (set `self.Timer` 0.0)
  (set `self.MinColor` 0.004636))