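; Controller for a three-stage musical puzzle that opens a pillar for each correctly entered melody and finally opens a bridge.
; Incoming notes route by melody number to that stage's note array, advancing a shared counter or resetting it on a mistake.
; A completed sequence plays the melody, opens its pillar after timed delays, then loads the next sound or opens the bridge.
; A separate event plays the current melody, guarded against overlapping playback.
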(event `SetMelody2`
  ;[1 1 1] Change melodies
  (`AudioComponent.SetSound` (`self.MelodyPlayer`) "/Game/Sounds/Melodies/S_Melody_2.S_Melody_2"))

(event `PlayMelody_Event`
  ;[1 1 1] Plays the current melody loaded.
  (if (`self.AlreadyPlayed`)
    _
    (elif (not (`self.NotePlaying`))
      (`AudioComponent.Play` (`self.MelodyPlayer`) 0.0)
      (set `self.AlreadyPlayed` true))))

(event `AddNote_Event`
  (params (NoteSent :type Integer))
  ;[1 1 1] Switch between melodies.
  (switch `int` (`self.MelodyNumber`)
    (:`1`
      (`self.AddNoteNivell1` NoteSent))
    (:`2`
      (`self.AddNoteNivell2` NoteSent))
    (:`3`
      (`self.AddNoteNivell3` NoteSent))))

(event `SetMelody3`
  ;[1 1 1] Change melodies
  (`AudioComponent.SetSound` (`self.MelodyPlayer`) "/Game/Sounds/Melodies/S_Melody_3.S_Melody_3"))

(event `self.MelodyPlayer.OnAudioFinished`
  ;[1 1 1] Plays the current melody loaded.
  (set `self.NotePlaying` false)
  (set `self.AlreadyPlayed` false))

(event `AddNoteNivell1`
  (params (Note :type Integer))
  (bind _notecounterinarray (`self.NoteCounterInArray`))
  ;[1 1 1] Melody 1 sequence
  (if (== Note (`|GetArrayItem` (`self.Nivell1Notes`) (`self.NoteCounterInArray`)))
    (if (== (- (`KismetArrayLibrary.Array_Length` (`self.Nivell1Notes`)) 1) _notecounterinarray)
      (set `self.NotePlaying` true)
      (`KismetSystemLibrary.Delay` 2.0)
      (`AudioComponent.Play` (`self.MelodyPlayer`) 0.0)
      (`KismetSystemLibrary.Delay` (+ (`SoundBase.Duration` (`AudioComponent.Sound` (`self.MelodyPlayer`))) 0.5))
      (`/Game/Blueprints/BP_MovingPilar.OpenPilar_Event` (`self.Pilar1`))
      (set `self.MelodyNumber` 2)
      (`self.SetMelody2`)
      (else
        (bind _result (`/Engine/EditorBlueprintResources/StandardMacros.IncrementInt` _notecounterinarray)
          (:`  `
            (set `self.NoteCounterInArray` _result)))))
    (else
      (set `self.NoteCounterInArray` 0))))

(event `AddNoteNivell2`
  (params (Note :type Integer))
  (bind _notecounterinarray (`self.NoteCounterInArray`))
  ;[1 1 1] Melody 2 sequence
  (if (== Note (`|GetArrayItem` (`self.Nivell2Notes`) (`self.NoteCounterInArray`)))
    (if (== (- (`KismetArrayLibrary.Array_Length` (`self.Nivell2Notes`)) 1) _notecounterinarray)
      (set `self.NotePlaying` true)
      (`KismetSystemLibrary.Delay` 2.0)
      (`AudioComponent.Play` (`self.MelodyPlayer`) 0.0)
      (`KismetSystemLibrary.Delay` (+ (`SoundBase.Duration` (`AudioComponent.Sound` (`self.MelodyPlayer`))) 0.5))
      (`/Game/Blueprints/BP_MovingPilar.OpenPilar_Event` (`self.Pilar2`))
      (set `self.MelodyNumber` 3)
      (`self.SetMelody3`)
      (else
        (bind _result (`/Engine/EditorBlueprintResources/StandardMacros.IncrementInt` _notecounterinarray)
          (:`  `
            (set `self.NoteCounterInArray` _result)))))
    (else
      (set `self.NoteCounterInArray` 0))))

(event `AddNoteNivell3`
  (params (Note :type Integer))
  (bind _notecounterinarray (`self.NoteCounterInArray`))
  ;[1 1 1] Melody 3 sequence
  (if (== Note (`|GetArrayItem` (`self.Nivell3Notes`) (`self.NoteCounterInArray`)))
    (if (== (- (`KismetArrayLibrary.Array_Length` (`self.Nivell3Notes`)) 1) _notecounterinarray)
      (set `self.NotePlaying` true)
      (`KismetSystemLibrary.Delay` 2.0)
      (`AudioComponent.Play` (`self.MelodyPlayer`) 0.0)
      (`KismetSystemLibrary.Delay` (+ (`SoundBase.Duration` (`AudioComponent.Sound` (`self.MelodyPlayer`))) 0.5))
      (`/Game/Blueprints/BP_MovingPilar.OpenPilar_Event` (`self.Pilar3`))
      (`KismetSystemLibrary.Delay` (`SoundBase.Duration` (`AudioComponent.Sound` (`self.GetComponentByClass` (`self.Pilar3`) "/Script/Engine.AudioComponent"))))
      (`/Game/Blueprints/BP_Bridge.Open_Bridge` (`self.Bridge`))
      (else
        (bind _result (`/Engine/EditorBlueprintResources/StandardMacros.IncrementInt` _notecounterinarray)
          (:`  `
            (set `self.NoteCounterInArray` _result)))))
    (else
      (set `self.NoteCounterInArray` 0))))

(fn `UserConstructionScript`
  (set `self.MelodyNumber` 1)
  (set `self.AlreadyPlayed` false)
  (set `self.OnErrorAnimation` false)
  (set `self.NoteCounterInArray` 0)
  (set `self.NotePlaying` false))