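; PlataformaVerda is a green platform Blueprint that wiggles when something enters its Box trigger and is released to physics when it leaves.
; Begin overlap replays the Wiggle timeline, which moves the actor to the X and Y saved by the construction script, with Z set directly from the curve, not offset.
; End overlap enables physics simulation on the Cube; neither event filters the overlapping actor.
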(event `self.Box.OnComponentEndOverlap`
  (params (OverlappedComponent :type "PrimitiveComponent Object Reference") (OtherActor :type "Actor Object Reference") (OtherComp :type "PrimitiveComponent Object Reference") (OtherBodyIndex :type Integer))
  (`PrimitiveComponent.SetSimulatePhysics` (`self.Cube`) true))

(event `self.Box.OnComponentBeginOverlap`
  (params (OverlappedComponent :type "PrimitiveComponent Object Reference") (OtherActor :type "Actor Object Reference") (OtherComp :type "PrimitiveComponent Object Reference") (OtherBodyIndex :type Integer) (bFromSweep :type Boolean) (SweepResult :type "HitResult Structure (by ref)"))
  (bind (_direction _wigglef) (`Timeline|Wiggle` :!via `PlayFromStart`)
    (:`Update`
      (`self.K2_SetActorRelativeLocation` (`KismetMathLibrary.MakeVector` (.x (`self.InitialLocation`)) (.y (`self.InitialLocation`)) _wigglef)))))

(fn `UserConstructionScript`
  (set `self.InitialLocation` (`self.K2_GetActorLocation`)))