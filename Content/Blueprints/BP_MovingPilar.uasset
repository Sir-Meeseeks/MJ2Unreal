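; BP_MovingPilar is a pillar actor that slides along the Y axis to open and close when its custom events are called.
; The construction script caches the world location, which the PilarYMove timeline offsets in Y and applies as the actor's relative location.
; OpenPilar_Event plays SFXPilar and runs the timeline from the start.
; ClosePilar_Event reverses it from the end without triggering the sound.
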(event `OpenPilar_Event`
  (`AudioComponent.Play` (`self.SFX_Pilar`) 0.0)
  (bind (_direction _move_y_axis) (`Timeline|PilarYMove` :!via `PlayFromStart` :!label _label)
    (:`Update`
      (`self.K2_SetActorRelativeLocation` (`KismetMathLibrary.MakeVector` (.x (`self.InitialPosition`)) (+ _move_y_axis (.y (`self.InitialPosition`))) (.z (`self.InitialPosition`)))))))

(event `ClosePilar_Event`
  (goto _label :!via `ReverseFromEnd`))

(fn `UserConstructionScript`
  (set `self.InitialPosition` (`self.K2_GetActorLocation`)))