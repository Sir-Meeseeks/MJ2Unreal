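; BP_DoorSeal_Y is a door seal actor that spins about its local Y axis and then opens a double door.
; Its Rotate event plays the seal sound and runs a timeline, applying the float track as a local rotation delta each update.
; When the timeline finishes, it plays the sound again and calls OpenDoor on the left and right wings.
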(event `Rotate`
  (`AudioComponent.Play` (`self.SFX_Seal`) 0.0)
  (bind (_direction _rotationfloat) (`Timeline|Rotation` :!via `PlayFromStart`)
    (:`Update`
      (`self.K2_AddActorLocalRotation` (`KismetMathLibrary.RotatorFromAxisAndAngle` (0.0 1.0 0.0) _rotationfloat)))
    (:`Finished`
      (`AudioComponent.Play` (`self.SFX_Seal`) 0.0)
      (`/Game/Blueprints/BP_Door_LeftWing_Y.OpenDoor` (`self.LeftWing`))
      (`/Game/Blueprints/BP_Door_RightWing_Y.OpenDoor` (`self.RightWing`)))))

(fn `UserConstructionScript`)