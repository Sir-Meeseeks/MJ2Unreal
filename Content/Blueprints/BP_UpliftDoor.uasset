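; BP_UpliftDoor is a door that toggles between lowered and raised positions through vertical movement.
; MoveDoor_Event flips DoorIsUp and plays the DoorUp timeline from start to open or reverses it from end to close.
; The timeline's float offsets the static mesh's relative Z from InitialPos, the actor's world location cached in the construction script.
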(event `MoveDoor_Event`
  (if (`self.DoorIsUp`)
    (set `self.DoorIsUp` false)
    (bind (_direction _movedoorfloat) (`Timeline|DoorUp` :!via `ReverseFromEnd` :!label _label)
      (:`Update`
        (`SceneComponent.K2_SetRelativeLocation` (`self.StaticMeshComponent`) (`KismetMathLibrary.MakeVector` (.x (`self.InitialPos`)) (.y (`self.InitialPos`)) (+ _movedoorfloat (.z (`self.InitialPos`)))) false false)))
    (else
      (set `self.DoorIsUp` true)
      (goto _label :!via `PlayFromStart`))))

(fn `UserConstructionScript`
  (set `self.DoorIsUp` false)
  (set `self.InitialPos` (`self.K2_GetActorLocation`)))