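; Game mode that respawns the third-person character after it is destroyed and resets the level's platforms.
; BeginPlay and the Respawn event bind to the player character's OnDestroyed, which after a short delay spawns and possesses a new character.
; It then restarts all correct and incorrect platforms; SetSpawnPoint updates only the spawn location.
; The respawn sequence itself does not rebind OnDestroyed on the new character.
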(event `Respawn`
  (bind _asbp_third_person_character (cast `/Game/Blueprints/BP_ThirdPersonCharacter` (`GameplayStatics.GetPlayerCharacter` 0) :!label _label))
  (add `self.OnDestroyed` _asbp_third_person_character (delegate `OnDestroyed_Event`)))

(event `self.ReceiveBeginPlay`
  (goto _label))

(event `OnDestroyed_Event` :!signature `self.OnDestroyed`
  (params (DestroyedActor :type "Actor Object Reference"))
  (`KismetSystemLibrary.Delay` 2.0)
  (bind _returnvalue (`|SpawnActorFromClass` "/Game/Blueprints/BP_ThirdPersonCharacter.BP_ThirdPersonCharacter_C" (`self.SpawnTransform`) "AdjustIfPossibleButAlwaysSpawn" "OverrideRootScale" null null))
  (`Controller.Possess` (`GameplayStatics.GetPlayerController` 0) _returnvalue)
  (`|ExecutionSequence`
    (:`then_0`
      (bind _outactors (`GameplayStatics.GetAllActorsOfClass` "/Game/Blueprints/BP_Platform_Correct.BP_Platform_Correct_C"))
      (for _array_element _outactors
        (`/Game/Blueprints/BP_Platform_Correct.Restart` _array_element)))
    (:`then_1`
      (bind _outactors_2 (`GameplayStatics.GetAllActorsOfClass` "/Game/Blueprints/BP_Platform_Incorrect.BP_Platform_Incorrect_C"))
      (for _array_element_2 _outactors_2
        (`/Game/Blueprints/BP_Platform_Incorrect.Restart` _array_element_2)))))

(event `SetSpawnPoint`
  (params (NewPoint :type "Vector Structure"))
  ;[1 1 1] SetSpawnPoint
  (set `self.SpawnTransform` (`KismetMathLibrary.MakeTransform` NewPoint (.rotation (`self.SpawnTransform`)) (.scale (`self.SpawnTransform`)))))

(fn `UserConstructionScript`)