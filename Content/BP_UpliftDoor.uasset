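; BP_UpliftDoor is a door actor that toggles between raised and lowered on the F key or through MoveDoor_Event.
; A DoorIsUp flag, initialized false in the construction script, picks whether the DoorUp timeline plays forward or reverses.
; The timeline's MoveDoor track sets the static mesh's relative location.
; A custom event enables player 0 input, and Tick re-sets the actor's location to its current value.
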(event `CustomEvent`
  (params (DeltaSeconds :type "Float (double-precision)"))
  (`self.EnableInput` (`GameplayStatics.GetPlayerController` 0)))

(event `Key|F`
  (params (Key :type "Key Structure"))
  (:`Pressed`
    (if (`self.DoorIsUp`) :!label _label
      (set `self.DoorIsUp` false)
      (bind (_direction _movedoor) (`Timeline|DoorUp` :!via `ReverseFromEnd` :!label _label_2)
        (:`Update`
          (`SceneComponent.K2_SetRelativeLocation` (`self.StaticMeshComponent`) _movedoor false false)))
      (else
        (set `self.DoorIsUp` true)
        (goto _label_2 :!via `PlayFromStart`)))))

(event `MoveDoor_Event`
  (goto _label))

(event `self.ReceiveTick`
  (params (DeltaSeconds :type "Float (single-precision)"))
  (`self.K2_SetActorLocation` (`self.K2_GetActorLocation`)))

(fn `UserConstructionScript`
  (set `self.DoorIsUp` false))